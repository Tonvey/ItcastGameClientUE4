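; Bullet is a networked skill projectile that reports its hits on players.
; The construction script records its spawn position, and Tick destroys it once it travels beyond a fixed maximum range.
; Hitting anything but its owner destroys it; a PlayerBase target also triggers a SkillContact message with source, target, skill and bullet IDs, target HP and hit location, pushed to the network controller.
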(event `self.ReceiveBeginPlay`)

(event `self.ReceiveHit`
  (params (MyComp :type "PrimitiveComponent Object Reference") (Other :type "Actor Object Reference") (OtherComp :type "PrimitiveComponent Object Reference") (bSelfMoved :type Boolean) (HitLocation :type "Vector Structure") (HitNormal :type "Vector Structure") (NormalImpulse :type "Vector Structure") (Hit :type "HitResult Structure (by ref)"))
  (if (not (== Other (`self.GetOwner`)))
    (`self.K2_DestroyActor`)
    (bind _asplayer_base (cast `PlayerBase` Other))
    (bind _returnvalue (`NetworkMessageFactoryUtil.MakePositionPack` (`PlayerBase.HP` _asplayer_base) HitLocation))
    (bind _returnvalue_2 (`NetworkMessageFactoryUtil.MakeSkillContact` (`self.pid`) (`PlayerBase.mPid` _asplayer_base) (`self.skillId`) (`self.bulletId`) _returnvalue))
    (bind _returnvalue_3 (`NetworkMessageFactoryUtil.GetNetworkControllerInstance`))
    (`NetworkController.PushMsg` _returnvalue_3 _returnvalue_2)))

(event `self.ReceiveTick`
  (params (DeltaSeconds :type "Float (single-precision)"))
  (if (> (`KismetMathLibrary.Vector_Distance` (`self.BornPosition`) (`self.K2_GetActorLocation`)) 10000.0)
    (`self.K2_DestroyActor`)))

(fn `UserConstructionScript`
  (set `self.BornPosition` (`self.K2_GetActorLocation`)))