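; AICompetitor is a character representing a competitor, driven by sync events for movement, name, HP and skills.
; It creates a PlayerHUD widget, reprojects it above the capsule each Tick and removes it on destruction.
; Movement sync stores a destination, flags movement and snaps yaw.
; Skill triggers call CallOnFire and spawn a Bullet, but the nodes assigning its Pid, BulletId and SkillId are disconnected.
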(event `self.ReceiveTick`
  (params (DeltaSeconds :type "Float (single-precision)"))
  (`self.UpdateHub`))

(event `self.ReceiveBeginPlay`
  (`CharacterMovementComponent.SetMovementMode` (`self.CharacterMovement`) "MOVE_Walking" 0)
  (bind _returnvalue (`|CreateWidget` "/Game/UI/PlayerHUD.PlayerHUD_C"))
  (bind _output_get (set `self.Hub` _returnvalue))
  (`UserWidget.AddToViewport` _output_get 0))

(event `SyncGroundPositionTo_1`
  (params (_destination :type "Vector Structure") (_direction :type "Float (double-precision)"))
  (set `self.DestGroundtLocation` _destination)
  (set `self.InMoving` true)
  (`self.K2_SetActorRotation` (`KismetMathLibrary.MakeRotator` 0.0 0.0 _direction)))

(event `UpdateNameAndHp_1`
  (params (_name :type String) (_maxHp :type Integer) (_hp :type Integer))
  (`/Game/UI/PlayerHUD.UpdateUI` (`self.Hub`) _name _maxHp _hp))

(event `UpdateUIName_1`
  (params (_name :type String))
  (`/Game/UI/PlayerHUD.UpdateName` (`self.Hub`) _name))

(event `UpdateUIHp_1`
  (params (_maxHp :type Integer) (_hp :type Integer))
  (`/Game/UI/PlayerHUD.UpdateHP` (`self.Hub`) _maxHp _hp))

(event `self.ReceiveDestroyed`
  (`Widget.RemoveFromParent` (`self.Hub`))
  (set `self.Hub` null))

(event `ReceiveSkillTrigger_1`
  (params (skillId :type Integer) (bulletId :type Integer) (skillPos :type "Vector Structure") (bulletVelocity :type "Vector Structure (by ref)"))
  (`self.OnFire`)
  (bind _returnvalue (`|SpawnActorFromClass` "/Game/BluePrints/Bullet.Bullet_C" (`KismetMathLibrary.MakeTransform` skillPos (`self.K2_GetActorRotation`)) "AdjustIfPossibleButAlwaysSpawn" "OverrideRootScale" self null)))

(fn `UpdateHub`
  (bind _hub (`self.Hub`))
  (`/Engine/EditorBlueprintResources/StandardMacros.IsValid` _hub
    (:`Is Valid`
      (`/Game/UI/PlayerHUD.UpdateToScreenPosition` _hub (`PlayerCameraManager.GetCameraLocation` (`PlayerController.PlayerCameraManager` (`GameplayStatics.GetPlayerController` 0))) (+ (`self.K2_GetActorLocation`) (`KismetMathLibrary.MakeVector` 0.0 0.0 (+ (`CapsuleComponent.GetScaledCapsuleHalfHeight` (`self.CapsuleComponent`)) (`self.HubOffsetZ`))))))))

(fn `UserConstructionScript`)