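; Competitor is a walking character with a name text, moved by synced ground positions, likely standing in for another player.
; SyncGroundPositionto stores a destination, flags movement and immediately sets the actor's yaw to the given direction.
; While moving, Tick logs the remaining distance and feeds movement input toward the destination, snapping onto it and stopping once close.
; The construction script assigns the name text and mesh components to member variables.
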(event `self.ReceiveTick`
  (params (DeltaSeconds :type "Float (single-precision)"))
  (bind _returnvalue (`self.GetPlayerGroundLocation`))
  (bind _destgroundtlocation (`self.DestGroundtLocation`))
  (bind _returnvalue_2 (`KismetMathLibrary.Vector_Distance` _destgroundtlocation _returnvalue))
  (if (`self.InMoving`)
    (`VisualLoggerKismetLibrary.LogText` null (`KismetStringLibrary.Conv_DoubleToString` _returnvalue_2) "CompetitorDistance" true)
    (if (<= _returnvalue_2 20.0)
      (`self.SetPlayerGroundLocation` (`self.DestGroundtLocation`))
      (set `self.InMoving` false)
      (else
        (`self.AddMovementInput` (- _destgroundtlocation _returnvalue))))))

(event `self.ReceiveBeginPlay`
  (`CharacterMovementComponent.SetMovementMode` (`self.CharacterMovement`) "MOVE_Walking" 0))

(event `self.SyncGroundPositionTo`
  (params (_destination :type "Vector Structure") (_direction :type "Float (single-precision)"))
  (set `self.DestGroundtLocation` _destination)
  (set `self.InMoving` true)
  (`self.K2_SetActorRotation` (`KismetMathLibrary.MakeRotator` 0.0 0.0 _direction)))

(fn `UserConstructionScript`
  (set `self.mPlayerNameTextComp` (`self.PlayerNameText`))
  (set `self.mPlayerMeshComp` (`self.Mesh`)))